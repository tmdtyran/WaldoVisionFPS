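; BP_ShooterHUD is the shooter's HUD Blueprint, managing the main gameplay widget and a kit selection screen.
; On BeginPlay it creates WBP_Main for the owning player controller, adds it to the viewport and refreshes its abilities.
; ShowKits lazily creates and caches WBP_KitSelection before adding it to the viewport, and HideKits removes it from its parent.
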(event Custom|ShowKits
  (bind _selectionkit (Variables|Default|GetSelectionKit)
    (:then
      _)
    (:else
      (bind _returnvalue (UserInterface|CreateWidget "/Game/UI/WBP_KitSelection.WBP_KitSelection_C"))
      (Variables|Default|SetSelectionKit _returnvalue)))
  (UserInterface|Viewport|AddtoViewport _selectionkit 0))

(event Custom|HideKits
  (bind _selectionkit (Variables|Default|GetSelectionKit)
    (:then
      (Widget|RemovefromParent _selectionkit))
    (:else)))

(event EventBeginPlay
  (bind _returnvalue (UserInterface|CreateWidget "/Game/UI/WBP_Main.WBP_Main_C" (Game|Player|GetOwningPlayerController)))
  (bind _output_get (Variables|Default|SetMainWidget _returnvalue))
  (UserInterface|Viewport|AddtoViewport _output_get 0)
  (Default|UpdateAbilities _returnvalue 0.0 0.0 0.0 0.0))

(fn ConstructionScript)