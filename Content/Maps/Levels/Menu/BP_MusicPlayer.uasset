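; Menu-level actor that plays music through a media player shared by the shooter game instance.
; On begin play it routes that player into its media sound component, listens for media-opened events, and tells the game instance to update the music file.
; When media opens, it calls Play, retrying every second until playback succeeds.
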(event Custom|OnOppened
  (params (OpenedUrl :type String))
  (bind _returnvalue (Media|MediaPlayer|Play (Variables|Default|GetMusic%20Player) :!class /Script/MediaAssets.MediaPlayer :!label _label))
  (if (not _returnvalue)
    (Utilities|FlowControl|Delay 1.0)
    (goto _label)))

(event EventBeginPlay
  (bind _asbp_shooter_game_instance (Utilities|Casting|CastToBP_ShooterGameInstance (Game|GetGameInstance)))
  (bind _output_get (Variables|Default|SetMusic%20Player (Variables|/Game/Maps/Modules/BP_ShooterGameInstance.BP_ShooterGameInstance_C|GetMusicPlayer _asbp_shooter_game_instance)))
  (Media|MediaSoundComponent|SetMediaPlayer (Variables|Default|GetMediaSound) _output_get)
  (Media|MediaPlayer|BindEventtoOnMediaOpened _output_get (delegate Custom|OnOppened))
  (Default|UpdateMusicFile _asbp_shooter_game_instance))

(event Collision|EventActorBeginOverlap
  (params (OtherActor :type Actor%20Object%20Reference)))

(event EventTick
  (params (DeltaSeconds :type Float%20%28single-precision%29)))

(fn ConstructionScript)