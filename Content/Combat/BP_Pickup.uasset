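; BP_Pickup is a pickup actor Blueprint in the Combat folder that appears to serve as an overridable base.
; Interaction range enter and exit events forward to ComponentInteraction's overlap handlers.
; CallStart passes a type to SpawnDespawnManager, and another event destroys a given widget component if valid.
; Construction calls an empty UpdateData hook, while getters expose name and thumbnail, with the mesh getter returning nothing.
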(event EventBeginPlay
  (if (Utilities|IsValid 0)
    _))

(event EventOnInteractionRangeExit
  (Default|OnEndOverlap (Variables|Default|GetComponent_Interaction)))

(event EventDestroyWidgetComponent
  (params (Widget%20Component :type Widget%20Component%20Object%20Reference))
  (Utilities|IsValid Widget%20Component
    (:Is%20Valid
      (Components|DestroyComponent Widget%20Component))))

(event EventCallStart
  (params (Type :type E_SpawnType%20Enum :default "NewEnumerator1"))
  (Default|Start (Variables|Default|GetSpawn_DespawnManager) Type))

(event EventOnInteractionRangeEntered
  (params (Pawn :type Pawn%20Object%20Reference) (Other%20Component :type Primitive%20Component%20Object%20Reference))
  (Default|OnBeginOverlap (Variables|Default|GetComponent_Interaction) Pawn Other%20Component))

(fn ConstructionScript
  (|CallParentFunction)
  (CallFunction|UpdateData))

(fn UpdateData)

(fn GetMeshBP
  (return 0))

(fn GetNameBP
  (return (Variables|Default|GetName)))

(fn GetThumbnailBP
  (return (Variables|Default|GetThumbnail)))