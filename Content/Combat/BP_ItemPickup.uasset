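; Pickup item for combat that switches between Dropped and Equipped states and carries either a skeletal or static mesh.
; The ItemState RepNotify toggles mesh physics and collision along with the interaction box's overlap.
; Interaction and pickup equip it, with pickup also caching the owning character; dropping clears that owner.
; Construction registers meshes with SpawnDespawnManager for dissolve and sets up the Pickup prompt on ComponentInteraction.
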(event Custom|OnPickedUp
  (Development|PrintString "should be server")
  (CallFunction|SetItemState "NewEnumerator1")
  (bind _asbp_third_person_character (Utilities|Casting|CastToBP_ThirdPersonCharacter (Components|GetOwner)))
  (bind _output_get (Variables|Default|SetOwnerCharacter _asbp_third_person_character))
  (CallFunction|CSetOwnerCharacter _output_get))

(event Custom|OnDropped
  (CallFunction|SetItemState "NewEnumerator0")
  (Variables|Default|SetOwnerCharacter 0))

(event Custom|C_SetOwnerCharacter
  (params (OwnerCharacter :type BP%20Third%20Person%20Character%20Object%20Reference))
  (Variables|Default|SetOwnerCharacter OwnerCharacter))

(event EventBeginPlay
  (|CallParentFunction)
  (CallFunction|SetItemState "NewEnumerator0"))

(event EventUpdateCollisionBP
  (params (State :type E_ItemState%20Enum :default "NewEnumerator0"))
  (CallFunction|SetItemState State))

(event EventUpdateRootComponentsAttach
  (params (ParentAttach :type Scene%20Component%20Object%20Reference) (Socket :type Name :default "None"))
  (CallFunction|UpdateRootStaticComponentsAttach (Variables|Default|GetSpawn_DespawnManager) ParentAttach Socket (Utilities|Array|MakeArray (Variables|Default|GetStaticMesh))))

(event EventOnInteracted
  (params (Actor :type Actor%20Object%20Reference))
  (CallFunction|SetItemState "NewEnumerator1"))

(fn ConstructionScript
  (bind _spawn_despawnmanager (Variables|Default|GetSpawn_DespawnManager))
  (|CallParentFunction)
  (Variables|/Game/Combat/Framework/ComponentsLibrary/Spawn_DespawnManager/BC_SpawnDespawnManager.BC_SpawnDespawnManager_C|SetDissolveStaticMeshes _spawn_despawnmanager (Utilities|Array|MakeArray (Utilities|Struct|MakeS_MoveStaticMesh (Variables|Default|GetStaticMesh) 0 "None")))
  (Variables|/Game/Combat/Framework/ComponentsLibrary/Spawn_DespawnManager/BC_SpawnDespawnManager.BC_SpawnDespawnManager_C|SetDissolveSkeletalMeshes _spawn_despawnmanager (Utilities|Array|MakeArray (Utilities|Struct|MakeS_MoveSkeletalMesh (Variables|Default|GetSkeletalMesh) (Variables|Default|GetStaticMesh) "None")))
  (Variables|/Game/Combat/Framework/ComponentsLibrary/InteractionSystem/Component_Interaction.Component_Interaction_C|SetSceneComponent (Variables|Default|GetComponent_Interaction) (Utilities|Map|MakeMap (Variables|Default|GetBox) (Utilities|Struct|MakeOverlapSettings "Pickup" "F" (Variables|Default|GetStaticMesh) "None"))))

(fn SetItemState
  (params (NewWeaponState :type E_ItemState%20Enum :default "NewEnumerator0"))
  (bind _output_get (Variables|Default|SetItem%20State NewWeaponState)))

(fn Drop
  (CallFunction|SetItemState "NewEnumerator0"))

(fn CreateDynamicMaterial
  (params (Mesh :type Mesh%20Component%20Object%20Reference)))

(fn OnRepItemState
  (bind _staticmesh (Variables|Default|GetStaticMesh))
  (switch Utilities|FlowControl|Switch|SwitchonE_ItemState (Variables|Default|GetItem%20State)
    (:NewEnumerator0
      (Collision|SetCollisionProfileName (Variables|Default|GetBox) "OverlapAllDynamic" true :!class /Script/Engine.PrimitiveComponent)
      (Collision|SetCollisionProfileName _staticmesh "DroppedItem" true :!class /Script/Engine.PrimitiveComponent)
      (Physics|SetSimulatePhysics _staticmesh true))
    (:NewEnumerator1
      (Physics|SetSimulatePhysics _staticmesh false)
      (Collision|SetCollisionProfileName (Variables|Default|GetBox) "NoCollision" true :!class /Script/Engine.PrimitiveComponent)
      (Collision|SetCollisionProfileName _staticmesh "NoCollision" true :!class /Script/Engine.PrimitiveComponent))))

(fn GetMeshBP
  (return (select (Utilities|IsValid (Components|SkeletalMesh|GetSkeletalMeshAsset (Variables|Default|GetSkeletalMesh))) (Variables|Default|GetSkeletalMesh) (Variables|Default|GetStaticMesh))))