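; Grenade explosion actor for frag, impact and flash types that deals distance-scaled damage on spawn, then destroys itself.
; BeginPlay leaves a decal, sphere-overlaps nearby actors and line-traces to their mesh bones, using only the head for flash, so cover blocks damage.
; The nearest visible bone sets the damage percent sent by message, though that distance never resets between actors.
; A radial impulse fires before destruction; debug traces and prints remain active.
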(event EventBeginPlay
  (bind _array (Utilities|Array|MakeArray "spine_02" "spine_01" "pelvis" "head" "lowerarm_l" "lowerarm_r" "thigh_l" "thigh_r" "foot_l" "foot_r"))
  (bind _defaultsceneroot1 (Variables|Default|GetDefaultSceneRoot1))
  (bind _grenadetype (Variables|Default|GetGrenadeType))
  (bind _defaultsceneroot1_2 (Variables|Default|GetDefaultSceneRoot1))
  (bind _returnvalue (Transformation|GetWorldLocation _defaultsceneroot1_2))
  (bind _returnvalue_2 (Transformation|GetWorldLocation _defaultsceneroot1))
  (switch Utilities|FlowControl|Switch|SwitchonE_GrenadeType (Variables|Default|GetGrenadeType)
    (:NewEnumerator0
      _)
    (:NewEnumerator5
      _)
    (:NewEnumerator1
      _))
  (Rendering|Decal|SpawnDecalatLocation "/Game/Combat/Pickables/Grenades/M_ExplosionDecal.M_ExplosionDecal" "200.000000,200.000000,200.000000" _returnvalue_2 "-90.000000,0.000000,0.000000" 4.0)
  (bind _outactors (Collision|SphereOverlapActors _returnvalue_2 (Variables|Default|GetIn%20Sphere%20Radius) (Utilities|Array|MakeArray "ObjectTypeQuery3" "ObjectTypeQuery6" "ObjectTypeQuery5") 0))
  (for (_array_element _array_index) _outactors
    (bind _mesh (Class|BPIPickupInterface|GetMeshBP(Message) _array_element))
    (Utilities|IsValid _mesh
      (:Is%20Valid
        (for _array_element_2 (Utilities|Select :Index _grenadetype :NewEnumerator0 _array :NewEnumerator5 _array :NewEnumerator1 (Utilities|Array|MakeArray "head") :NewEnumerator2 0 :NewEnumerator3 0 :NewEnumerator4 0)
          (bind (_outhit _returnvalue_3) (Collision|LineTraceByChannel _returnvalue (+ (Transformation|GetSocketLocation _mesh _array_element_2) (* (Math|Vector|GetUnitDirection(Vector) _returnvalue (Transformation|GetSocketLocation _mesh _array_element_2)) 2.0)) "TraceTypeQuery4" false (Variables|Default|GetCheckedActors) "Persistent"))
          (if (Math|Boolean|ANDBoolean _returnvalue_3 (== _array_element (.HitActor (Collision|BreakHitResult _outhit))) (Utilities|Name|Equal(Name) (.HitBoneName (Collision|BreakHitResult _outhit)) _array_element_2))
            (Variables|Default|SetActorHit true)
            (if (< (.Distance (Collision|BreakHitResult _outhit)) (Variables|Default|GetNearestDistance))
              (Variables|Default|SetNearestDistance (.Distance (Collision|BreakHitResult _outhit))))))
        (Utilities|Array|Add (Variables|Default|GetCheckedActors) _array_element)
        (if (Variables|Default|GetActorHit)
          (Class|CustomDammage|DammageGrenadeExplosion(Message) _array_element (- 1.0 (/ (Variables|Default|GetNearestDistance) (Variables|Default|GetIn%20Sphere%20Radius))) (Game|GetInstigatorController) _grenadetype _returnvalue_2)
          (Variables|Default|SetActorHit false)
          (Development|PrintString (Utilities|String|ToString(Float) (- 1.0 (/ (Variables|Default|GetNearestDistance) (Variables|Default|GetIn%20Sphere%20Radius)))))))))
  (Class|RadialForceComponent|FireImpulse (Variables|Default|GetRadialForce))
  (Actor|DestroyActor))

(fn ConstructionScript
  (Variables|Default|SetNearestDistance (Variables|Default|GetIn%20Sphere%20Radius)))