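; BP_Grenade is a pickable grenade actor, but most of its logic is disconnected.
; Only Detonate has live logic, playing a one-shot sound and oversized effect at the mesh.
; CallUnpin, Unpin, Hit and UpdateData are empty, and IsUnpinned always returns false.
; Unreachable nodes hold the type-based design: unpin montage with CCD and fuse delay, impact triggers, BP_FragExplosion spawning, and a timed attached smoke effect.
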(event Custom|Unpin)

(event Custom|Detonate
  (bind _staticmesh (Variables|Default|GetStaticMesh))
  (Utilities|FlowControl|DoOnce false
    (:Completed
      (Audio|PlaySoundatLocation 0 (Transformation|GetWorldLocation (Variables|Default|GetStaticMesh)) "0, 0, 0" 1.0 1.0 0.0 0 0 0 0)
      (Niagara|SpawnSystematLocation 0 (Transformation|GetWorldLocation _staticmesh) (Transformation|GetWorldRotation _staticmesh) "50.000000,50.000000,50.000000"))))

(event EventBeginPlay
  (|CallParentFunction) ; This node is disabled and will not be called.\nDrag off pins to build functionality.
)

(event EventCallUnpin)

(event EventTick
  (params (DeltaSeconds :type Float%20%28single-precision%29)))

(event Collision|EventActorBeginOverlap
  (params (OtherActor :type Actor%20Object%20Reference)))

(event Collision|EventHit
  (params (MyComp :type Primitive%20Component%20Object%20Reference) (Other :type Actor%20Object%20Reference) (OtherComp :type Primitive%20Component%20Object%20Reference) (bSelfMoved :type Boolean) (HitLocation :type Vector :default "0, 0, 0") (HitNormal :type Vector :default "0, 0, 0") (NormalImpulse :type Vector :default "0, 0, 0") (Hit :type Hit%20Result%20Structure%20%28by%20ref%29)))

(fn ConstructionScript
  (|CallParentFunction))

(fn UpdateData)

(fn IsUnpinned
  (return false))