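; Networked pickup weapon configured by type as rifle, sniper, shotgun or revolver, with switchable Blue, Green and Purple modes.
; A timer gates camera line-trace shots, which send type-based damage and bullet mode, then multicast tracer, impact and sound.
; Green and Purple charge over time while held, activate when full and revert to Blue when empty.
; Mode drives tracer and replicated overlay colors, while HUD events show ammo and charge.
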(event Custom|Shoot
  (params (True :type Boolean))
  ;[1 1 1] Shooting Logic
  (CallFunction|SRShoot True))

(event Custom|SR_Shoot
  (params (True :type Boolean))
  ;[1 1 1] Shooting Logic
  (bind _output_get (Variables|Default|SetWantsToShoot? True))
  (if True
    _
    (else
      (Variables|Default|SetReleasedTrigger true)))
  (if _output_get
    (if (and (> (Variables|Default|GetCurrentAmmo) 0) (Variables|Default|GetCanShoot))
      (if (Utilities|Time|IsValidTimerHandle (Variables|Default|GetShooterTimer))
        (CallFunction|ShootRifle)
        (else
          (bind _returnvalue (Utilities|Time|SetTimerbyEvent (EventDispatchers|CreateEvent :!event Custom|TryShoot) (Variables|Default|GetFireRate) true))
          (Variables|Default|SetShooterTimer _returnvalue)
          (CallFunction|TryShoot))))))

(event Custom|S_ActivatePurpleAbility
  ;[1 1 1] Ability Activation
  (if (Utilities|Enum|Equal(Enum) (Variables|Default|GetWeaponMode) "NewEnumerator2")
    (CallFunction|SActivateBlueAbility)
    (elif (== (Variables|Default|GetPurpleProgress) (Variables|Default|GetMaxPurpleProgress))
      (CallFunction|Shoot false)
      (Variables|Default|SetWeaponMode "NewEnumerator2")
      (Variables|Default|SetPurpleProgress 0.0)
      (CallFunction|MPlaySoundatWeaponLocation (Utilities|Select :Index (Variables|Default|GetWeaponType) :NewEnumerator0 "/Game/Sounds/RifleAbility.RifleAbility" :NewEnumerator1 "/Game/Sounds/SniperAbility.SniperAbility" :NewEnumerator2 "/Game/Sounds/ShotgunAbility.ShotgunAbility" :NewEnumerator3 "/Game/Sounds/RevolverAbility.RevolverAbility"))
      (CallFunction|CUpdateAbilityColor (Variables|Default|GetWeaponMode))
      (CallFunction|CUpdateAbilityWidget)
      (Utilities|FlowControl|Sequence
        (:then_0
          (Variables|Default|SetPreviousAmount (Variables|Default|GetCurrentAmmo)))
        (:then_1
          (switch Utilities|FlowControl|Switch|SwitchonE_WeaponType (Variables|Default|GetWeaponType)))
        (:then_2
          (CallFunction|UpdateAmmoCounter))))))

(event Custom|S_ActivateBlueAbility
  ;[1 1 1] Ability Activation
  (CallFunction|Shoot false)
  (Variables|Default|SetWeaponMode "NewEnumerator0")
  (CallFunction|CUpdateAbilityColor (Variables|Default|GetWeaponMode))
  (Variables|Default|SetCurrentAmmo (Variables|Default|GetPreviousAmount))
  (Utilities|FlowControl|Sequence
    (:then_0
      (switch Utilities|FlowControl|Switch|SwitchonE_WeaponType (Variables|Default|GetWeaponType)
        (:NewEnumerator0
          (Variables|Default|SetMaxAmmo 30))
        (:NewEnumerator1
          (Variables|Default|SetMaxAmmo 5))
        (:NewEnumerator2
          (Variables|Default|SetMaxAmmo 7))
        (:NewEnumerator3
          (Variables|Default|SetMaxAmmo 6))))
    (:then_1
      (CallFunction|UpdateAmmoCounter))))

(event Custom|C_RemoveAbilityWidget
  ;[1 1 1] Interaction
  ;;[1 1 1] Ability Widget
  (Variables|Default|SetMain%20Widget 0))

(event Custom|C_UpdateAbilityColor
  (params (WeaponMode :type E_WeaponMode%20Enum :default "NewEnumerator0"))
  (bind _main_widget (Variables|Default|GetMain%20Widget))
  ;[1 1 1] Ability Progress
  (Utilities|IsValid _main_widget
    (:Is%20Valid
      (Default|UpdateWeaponMode _main_widget WeaponMode)
      (Development|PrintString (Utilities|String|EnumtoString WeaponMode)))))

(event Custom|C_UpdateAmmoCounter
  (params (Current :type Integer) (Max :type Integer))
  ;[1 1 1] Ability Progress
  (Default|UpdateAmmoCounter (Variables|Default|GetMain%20Widget) Current Max))

(event Custom|UpdateAmmoCounter
  ;[1 1 1] Ability Progress
  (CallFunction|CUpdateAmmoCounter (Variables|Default|GetCurrentAmmo) (Variables|Default|GetMaxAmmo)))

(event Custom|S_Reload
  (CallFunction|Reload))

(event Custom|AddAbilityProgress
  (params (Green :type Boolean) (Purple :type Boolean) (Amount :type Float%20%28double-precision%29))
  ;[1 1 1] Ability Progress
  (Utilities|FlowControl|Sequence
    (:then_0
      (if Green
        (Variables|Default|SetGreenProgress (+ (Variables|Default|GetGreenProgress) Amount))))
    (:then_1
      (if Purple
        (Variables|Default|SetPurpleProgress (+ (Variables|Default|GetPurpleProgress) Amount))))
    (:then_2
      (CallFunction|CUpdateAbilityWidget))))

(event Custom|M_Impact
  (params (Location :type Vector) (Rotation :type Rotator))
  (Niagara|SpawnSystematLocation "/Game/VFX/Niagara_FX/ParticleSystems/PSN_Sparks_Surface.PSN_Sparks_Surface" Location Rotation "1.000000,1.000000,1.000000" true true "AutoRelease"))

(event Custom|M_Laser
  (params (EndLocation :type Vector))
  (bind _mesh (CallFunction|GetMeshBP))
  (bind _returnvalue (Niagara|SpawnSystematLocation "/Game/VFX/BulletTracers/NE_BaseTracer_System.NE_BaseTracer_System" (Transformation|GetSocketLocation _mesh "Muzzle") "0, 0, 0" "1.000000,1.000000,1.000000" true true "AutoRelease"))
  (Utilities|IsValid _returnvalue
    (:Is%20Valid
      (Niagara|SetNiagaraVariable(Vector3) _returnvalue "BeamEnd" (- EndLocation (Transformation|GetSocketLocation _mesh "Muzzle")))
      (Niagara|SetNiagaraVariable(LinearColor) _returnvalue "BeamColor" (Utilities|Select :Index (Variables|Default|GetWeaponMode) :NewEnumerator0 (Utilities|Struct|MakeLinearColor 0.0 0.0 1.0 1.0) :NewEnumerator1 (Utilities|Struct|MakeLinearColor 0.0 1.0 0.0 1.0) :NewEnumerator2 (Utilities|Struct|MakeLinearColor 1.0 0.0 1.0 1.0))))))

(event Custom|ShootRifle
  (bind _currentammo (Variables|Default|GetCurrentAmmo))
  (bind _ownercharacter (Variables|Default|GetOwnerCharacter))
  (bind _returnvalue (Pawn|GetControlRotation _ownercharacter :!class /Script/Engine.Pawn))
  (bind _followcamera (Variables|/Game/Characters/BP_ThirdPersonCharacter.BP_ThirdPersonCharacter_C|GetFollowCamera _ownercharacter))
  (bind _returnvalue_2 (Transformation|GetWorldLocation _followcamera))
  (bind _returnvalue_3 (Math|Vector|GetForwardVector _returnvalue))
  (bind _returnvalue_4 (* _returnvalue_3 10000))
  (bind _returnvalue_5 (+ _returnvalue_2 _returnvalue_4))
  (Utilities|FlowControl|Sequence
    (:then_0
      (Variables|Default|SetCanShoot false)
      (bind (_outhit _returnvalue_6) (Collision|LineTraceByChannel _returnvalue_2 _returnvalue_5 "TraceTypeQuery3" false (Utilities|Array|MakeArray _ownercharacter) "None" true (Utilities|Select :Index (Variables|Default|GetWeaponMode) :NewEnumerator0 "(R=0.000000,G=0.000000,B=1.000000,A=1.000000)" :NewEnumerator1 "(R=0.000000,G=1.000000,B=0.000000,A=1.000000)" :NewEnumerator2 "(R=0.694480,G=0.000000,B=1.000000,A=1.000000)") "(R=1.000000,G=0.000000,B=0.000000,A=1.000000)"))
      (if _returnvalue_6
        (Class|CustomDammage|DammageBullet(Message) (.HitActor (Collision|BreakHitResult _outhit)) (Utilities|Select :Index (Variables|Default|GetWeaponType) :NewEnumerator0 12.0 :NewEnumerator1 4e+01 :NewEnumerator2 (* (- 1.0 (Math|Float|MapRangeClamped (.Distance (Collision|BreakHitResult _outhit)) 1e+03 5e+03 0.0 0.9)) 8e+01) :NewEnumerator3 3e+01) 1.0 (.HitBoneName (Collision|BreakHitResult _outhit)) (Variables|Default|GetOwnerCharacter) (Variables|Default|GetWeaponMode))
        (CallFunction|MImpact (.Location (Collision|BreakHitResult _outhit)) (Math|Rotator|MakeRotfromX (.ImpactNormal (Collision|BreakHitResult _outhit))))
        (CallFunction|MLaser (.Location (Collision|BreakHitResult _outhit)))
        (else
          (CallFunction|MLaser _returnvalue_5))))
    (:then_1
      (Math|Integer|DecrementInt _currentammo
        (:%20%20
          (CallFunction|UpdateAmmoCounter)
          (if (and (== _currentammo 0) (Utilities|Enum|NotEqual(Enum) (Variables|Default|GetWeaponMode) "NewEnumerator0"))
            (CallFunction|SActivateBlueAbility)))))
    (:then_2
      (CallFunction|MPlaySoundatWeaponLocation "/Game/Sounds/laserShoot.laserShoot"))))

(event Custom|TryShoot
  ;[1 1 1] Shooting Logic
  (switch Utilities|FlowControl|Switch|SwitchonE_WeaponType (Variables|Default|GetWeaponType)
    (:NewEnumerator0
      (Variables|Default|SetCanShoot true)
      (if (Variables|Default|GetWantsToShoot?) :!label _label
        (if (and (> (Variables|Default|GetCurrentAmmo) 0) (Variables|Default|GetCanShoot))
          (if (Utilities|Time|IsValidTimerHandle (Variables|Default|GetShooterTimer))
            (CallFunction|ShootRifle)
            (else
              (bind _returnvalue (Utilities|Time|SetTimerbyEvent (EventDispatchers|CreateEvent :!event Custom|TryShoot) (Variables|Default|GetFireRate) true))
              (Variables|Default|SetShooterTimer _returnvalue)
              (CallFunction|TryShoot))))
        (else
          (Utilities|Time|ClearandInvalidateTimerbyHandle (Variables|Default|GetShooterTimer)))))
    (:NewEnumerator1
      (if (Variables|Default|GetReleasedTrigger) :!label _label_2
        (Variables|Default|SetCanShoot true)
        (Variables|Default|SetReleasedTrigger false)
        (else
          (goto _label))))
    (:NewEnumerator2
      (goto _label_2))
    (:NewEnumerator3
      (goto _label_2))))

(event Custom|S_CreateAbilityEvent
  ;[1 1 1] Ability Progress
  (bind _returnvalue (Utilities|Time|SetTimerbyEvent (delegate Custom|AddRegularAbilityProgress) 0.1 true))
  (Variables|Default|SetAbilityTimer _returnvalue))

(event Custom|AddRegularAbilityProgress
  ;[1 1 1] Ability Progress
  (switch Utilities|FlowControl|Switch|SwitchonE_WeaponMode (Variables|Default|GetWeaponMode)
    (:NewEnumerator0
      (Utilities|FlowControl|Sequence
        (:then_0
          (Variables|Default|SetGreenProgress (Math|Float|Clamp(Float) (+ (Variables|Default|GetGreenProgress) 0.1) 0.0 (Variables|Default|GetMaxGreenProgress)) :!label _label))
        (:then_1
          (Variables|Default|SetPurpleProgress (Math|Float|Clamp(Float) (+ (Variables|Default|GetPurpleProgress) 0.1) 0.0 (Variables|Default|GetMaxPurpleProgress)) :!label _label_2))
        (:then_2
          (CallFunction|CUpdateAbilityWidget :!label _label_3))))
    (:NewEnumerator1
      (Utilities|FlowControl|Sequence
        (:then_0
          (goto _label_2))
        (:then_1
          (goto _label_3))))
    (:NewEnumerator2
      (Utilities|FlowControl|Sequence
        (:then_0
          (goto _label))
        (:then_1
          (goto _label_3))))))

(event Custom|C_GetAbilityWidget
  ;[1 1 1] Interaction
  ;;[1 1 1] Ability Widget
  (bind _asplayer_controller (Utilities|Casting|CastToPlayerController (Pawn|GetController (Variables|Default|GetOwnerCharacter))))
  (bind _asbp_shooter_hud (Utilities|Casting|CastToBP_ShooterHUD (HUD|GetHUD _asplayer_controller)))
  (Variables|Default|SetMain%20Widget (Variables|/Game/Maps/Modules/BP_ShooterHUD.BP_ShooterHUD_C|GetMainWidget _asbp_shooter_hud)))

(event Custom|M_PlaySoundAtWeaponLocation
  (params (Sound :type Sound%20Base%20Object%20Reference))
  (Audio|PlaySoundatLocation Sound (.location (Transformation|GetSocketTransform (Variables|Default|GetStaticMesh) "None" "RTS_World")) "0, 0, 0" 1.0 1.0 0.0 "/Game/Sounds/NewSoundAttenuation.NewSoundAttenuation" 0 0 0))

(event Custom|C_UpdateAbilityWidget
  (bind _main_widget (Variables|Default|GetMain%20Widget))
  ;[1 1 1] Ability Progress
  (Utilities|IsValid _main_widget
    (:Is%20Valid
      (Default|UpdateAbilities _main_widget (Variables|Default|GetGreenProgress) (Variables|Default|GetPurpleProgress) (Variables|Default|GetMaxGreenProgress) (Variables|Default|GetMaxPurpleProgress)))))

(event Custom|S_ActivateGreenAbility
  ;[1 1 1] Ability Activation
  (if (Utilities|Enum|Equal(Enum) (Variables|Default|GetWeaponMode) "NewEnumerator1")
    (CallFunction|SActivateBlueAbility)
    (elif (== (Variables|Default|GetGreenProgress) (Variables|Default|GetMaxGreenProgress))
      (CallFunction|Shoot false)
      (Variables|Default|SetWeaponMode "NewEnumerator1")
      (Variables|Default|SetGreenProgress 0.0)
      (CallFunction|MPlaySoundatWeaponLocation (Utilities|Select :Index (Variables|Default|GetWeaponType) :NewEnumerator0 "/Game/Sounds/RifleAbility.RifleAbility" :NewEnumerator1 "/Game/Sounds/SniperAbility.SniperAbility" :NewEnumerator2 "/Game/Sounds/ShotgunAbility.ShotgunAbility" :NewEnumerator3 "/Game/Sounds/RevolverAbility.RevolverAbility"))
      (CallFunction|CUpdateAbilityColor (Variables|Default|GetWeaponMode))
      (CallFunction|CUpdateAbilityWidget)
      (Utilities|FlowControl|Sequence
        (:then_0
          (Variables|Default|SetPreviousAmount (Variables|Default|GetCurrentAmmo)))
        (:then_1
          (switch Utilities|FlowControl|Switch|SwitchonE_WeaponType (Variables|Default|GetWeaponType)
            (:NewEnumerator0
              (Variables|Default|SetCurrentAmmo 5)
              (Variables|Default|SetMaxAmmo 5))
            (:NewEnumerator1
              (Variables|Default|SetCurrentAmmo 1 :!label _label)
              (Variables|Default|SetCurrentAmmo 1))
            (:NewEnumerator2
              (goto _label))
            (:NewEnumerator3
              (goto _label))))
        (:then_2
          (CallFunction|UpdateAmmoCounter))))))

(event EventBeginPlay
  (bind _staticmesh (Variables|Default|GetStaticMesh))
  (bind _skeletalmesh (Variables|Default|GetSkeletalMesh))
  (|CallParentFunction)
  (bind _returnvalue (Rendering|Material|CreateDynamicMaterialInstance "/Game/Characters/M_Overlay_Inst.M_Overlay_Inst" "WeaponOverlay" "Transient" :!class /Script/Engine.KismetMaterialLibrary))
  (Variables|Default|SetOverlayMaterial _returnvalue)
  (Utilities|IsValid (Variables|/Script/Engine.StaticMeshComponent|GetStaticMesh _staticmesh)
    (:Is%20Valid
      (Rendering|Material|SetOverlayMaterial _staticmesh (Variables|Default|GetOverlayMaterial) :!class /Script/Engine.MeshComponent))
    (:Is%20Not%20Valid
      _))
  (Utilities|IsValid (Components|SkeletalMesh|GetSkeletalMeshAsset _skeletalmesh)
    (:Is%20Valid
      (Rendering|Material|SetOverlayMaterial _skeletalmesh (Variables|Default|GetOverlayMaterial) :!class /Script/Engine.MeshComponent))))

(event EventOnInteracted
  (params (Actor :type Actor%20Object%20Reference))
  ;[1 1 1] Interaction
  (Class|Pickups|CallPickupWeapon(Message) Actor self))

(event EventOnPickedUp
  ;[1 1 1] Interaction
  (|CallParentFunction)
  (CallFunction|SCreateAbilityEvent)
  (CallFunction|SCreateAbilityEvent)
  (CallFunction|CGetAbilityWidget)
  (CallFunction|UpdateAmmoCounter))

(event EventOnDropped
  ;[1 1 1] Interaction
  (|CallParentFunction)
  (Utilities|Time|ClearandInvalidateTimerbyHandle (Variables|Default|GetAbilityTimer))
  (Variables|Default|SetGreenProgress 0.0)
  (Variables|Default|SetPurpleProgress 0.0)
  (CallFunction|CUpdateAbilityWidget)
  (CallFunction|CRemoveAbilityWidget))

(fn ConstructionScript
  (bind _weapontype (Variables|Default|GetWeaponType))
  (|CallParentFunction)
  (bind _output_get (Variables|Default|SetMaxAmmo (Utilities|Select :Index _weapontype :NewEnumerator0 30 :NewEnumerator1 5 :NewEnumerator2 7 :NewEnumerator3 6)))
  (bind _output_get_2 (Variables|Default|SetCurrentAmmo (+ _output_get (Utilities|Select :Index _weapontype :NewEnumerator0 1 :NewEnumerator1 0 :NewEnumerator2 1 :NewEnumerator3 0))))
  (Variables|Default|SetPreviousAmount _output_get_2)
  (Variables|Default|SetFireRate (Utilities|Select :Index _weapontype :NewEnumerator0 0.1 :NewEnumerator1 1.0 :NewEnumerator2 0.2 :NewEnumerator3 0.4))
  (Components|StaticMesh|SetStaticMesh (Variables|Default|GetStaticMesh) (Utilities|Select :Index _weapontype :NewEnumerator0 "/Game/Combat/Weapons/Revolver/uploads_files_2656480_Revolver.uploads_files_2656480_Revolver" :NewEnumerator1 "/Game/Combat/Weapons/Revolver/uploads_files_2656480_Revolver.uploads_files_2656480_Revolver" :NewEnumerator2 "/Game/Combat/Weapons/Revolver/uploads_files_2656480_Revolver.uploads_files_2656480_Revolver" :NewEnumerator3 "/Game/Combat/Weapons/Revolver/uploads_files_2656480_Revolver.uploads_files_2656480_Revolver"))
  (Components|SkeletalMesh|SetSkeletalMeshAsset (Variables|Default|GetSkeletalMesh) (Utilities|Select :Index _weapontype :NewEnumerator0 0 :NewEnumerator1 0 :NewEnumerator2 0 :NewEnumerator3 0)))

(fn OnRepAbilityTimer)

(fn OnRepWeaponMode
  (bind _overlaymaterial (Variables|Default|GetOverlayMaterial)
    (:then
      (Rendering|Material|SetScalarParameterValue _overlaymaterial "ColorId" (Utilities|Select :Index (Variables|Default|GetWeaponMode) :NewEnumerator0 0.0 :NewEnumerator1 1.0 :NewEnumerator2 2.0) :!class /Script/Engine.MaterialInstanceDynamic))
    (:else)))

(fn Reload
  (bind _ownercharacter (Variables|Default|GetOwnerCharacter))
  (bind _weapontype (Variables|Default|GetWeaponType))
  (bind _output_get (LocalVariables|SetAvailable (Default|GetAmmoTypeAmount _ownercharacter _weapontype)))
  (bind _output_get_2 (LocalVariables|SetToLoadAmount (Math|Integer|Min(Integer) (- (+ (Variables|Default|GetMaxAmmo) (Math|Integer|SelectInt (Utilities|Select :Index _weapontype :NewEnumerator0 1 :NewEnumerator1 0 :NewEnumerator2 1 :NewEnumerator3 0) 0 (> (Variables|Default|GetCurrentAmmo) 0))) (Variables|Default|GetCurrentAmmo)) _output_get)))
  (Variables|Default|SetCurrentAmmo (+ (Variables|Default|GetCurrentAmmo) _output_get_2))
  (Default|SSetAmmoTypeAmount _ownercharacter _weapontype (- _output_get _output_get_2))
  (CallFunction|UpdateAmmoCounter)
  (Default|SUpdateAmmoDisplay (Variables|Default|GetOwnerCharacter)))